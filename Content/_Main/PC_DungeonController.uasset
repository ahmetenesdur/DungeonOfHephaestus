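; Player controller for the dungeon game that handles movement input for the controlled pawn.
; It caches the pawn on BeginPlay and checks that it is valid on each movement axis event.
; The forward/backward and right/left axes add movement input along the forward and right vectors of the pawn's full control rotation, without isolating yaw.
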(event `self.ReceiveBeginPlay`
  (set `self.PlayerPawn` (`self.K2_GetPawn`)))

(event `InputAxis|Move Forward / Backward`
  (params (AxisValue :type "Float (single-precision)"))
  (bind _playerpawn (`self.PlayerPawn`))
  (`self.PlayerPawn`
    (:`then`
      (`Pawn.AddMovementInput` _playerpawn (`KismetMathLibrary.GetForwardVector` (`Pawn.GetControlRotation` _playerpawn)) AxisValue false))
    (:`else`)))

(event `InputAxis|Move Right / Left`
  (params (AxisValue :type "Float (single-precision)"))
  (bind _playerpawn (`self.PlayerPawn`))
  (`self.PlayerPawn`
    (:`then`
      (`Pawn.AddMovementInput` _playerpawn (`KismetMathLibrary.GetRightVector` (`Pawn.GetControlRotation` _playerpawn)) AxisValue false))
    (:`else`)))

(fn `UserConstructionScript`)